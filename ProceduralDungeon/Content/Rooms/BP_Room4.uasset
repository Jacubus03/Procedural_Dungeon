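; BP_Room4 is a room actor with three doors, set up as child actor components.
; Its construction script casts each door's child actor to DoorBase and adds it to the Doors array.
; It also gathers every box component on the actor into the Colliders array.
; The event graph holds only disabled placeholder events, so this Blueprint adds no runtime logic of its own.
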(event EventBeginPlay)

(event Collision|EventActorBeginOverlap
  (params (OtherActor :type Actor%20Object%20Reference)))

(event EventTick
  (params (DeltaSeconds :type Float%20%28single-precision%29)))

(fn ConstructionScript
  (for _array_element (Utilities|Array|MakeArray (Variables|Default|GetBP_Door1) (Variables|Default|GetBP_Door2) (Variables|Default|GetBP_Door3))
    (bind _asdoor_base (Utilities|Casting|CastToDoorBase (Variables|/Script/Engine.ChildActorComponent|GetChildActor _array_element)))
    (Utilities|Array|Add (Variables|Default|GetDoors) _asdoor_base))
  (for _array_element_2 (Actor|GetComponentsByClass "/Script/Engine.BoxComponent")
    (Utilities|Array|Add (Variables|Default|GetColliders) _array_element_2)))